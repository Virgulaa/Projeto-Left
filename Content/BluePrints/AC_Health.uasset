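; Health component that manages player 0's health, damage feedback and death notification.
; SetHealth adds health up to a maximum or overwrites it, messages the AnimInstance about low health, and slows walking at the minimum threshold without restoring speed.
; SetDamage plays camera shake and a head-socket particle burst, then, only when OnlyHealth is true, subtracts damage through SetHealth and sends DeathMessage at zero.
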(event EventBeginPlay
  ;[1 1 1] Event BeginPlay
  (Variables|Default|SetCharacter (Game|GetPlayerCharacter 0)))

(event EventSetHealth
  (params (AddHealth :type Boolean) (NewHealth :type Float%20%28double-precision%29))
  (bind _character (Variables|Default|GetCharacter))
  (bind _charactermovement (Variables|/Script/Engine.Character|GetCharacterMovement _character))
  ;[1 1 1] Sistema De Vida
  (if AddHealth
    (Variables|Default|SetHealth (Math|Float|Min(Float) (+ NewHealth (Variables|Default|GetHealth)) (Variables|Default|GetMaxHealth)))
    (else
      (Variables|Default|SetHealth NewHealth)))
  (Class|CharacterInterface|DamegeAnimation(Message) (Components|SkeletalMesh|GetAnimInstance (Variables|/Script/Engine.Character|GetMesh _character)) (<= (Variables|Default|GetHealth) (Variables|Default|GetMinHealth)))
  (Variables|/Script/Engine.CharacterMovementComponent|SetMaxWalkSpeed _charactermovement (select (<= (Variables|Default|GetHealth) (Variables|Default|GetMinHealth)) 1e+01 (Variables|/Script/Engine.CharacterMovementComponent|GetMaxWalkSpeed _charactermovement))))

(event EventSetDamage
  (params (Damage :type Float%20%28double-precision%29) (OnlyHealth :type Boolean))
  (Variables|Default|SetLocalDamage Damage)
  ;[1 1 1] Efeitos Visuais De Dano
  (Class|MatineeCameraShake|StartMatineeCameraShake (Game|GetPlayerCameraManager 0) "/Game/BluePrints/CameraEffects/Damge_CS.Damge_CS_C" 5.0 "CameraLocal" "0, 0, 0")
  (Effects|SpawnEmitteratLocation "/Game/StarterContent/Particles/P_Explosion.P_Explosion" (Transformation|GetSocketLocation (Variables|/Script/Engine.Character|GetMesh (Variables|Default|GetCharacter)) "head"))
  (if OnlyHealth
    (if (<= (- (Variables|Default|GetHealth) (Variables|Default|GetLocalDamage)) 0.0)
      (CallFunction|SetHealth false 0.0)
      (Class|CharacterInterface|Death(Message) (Variables|Default|GetCharacter))
      (else
        (CallFunction|SetHealth false (- (Variables|Default|GetHealth) (Variables|Default|GetLocalDamage)))
        (Development|PrintString "Recebendo Dano" true true "(R=0.673585,G=1.000000,B=0.027282,A=1.000000)")))))